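; Interactive floor actor that shuttles its static mesh back and forth between its starting position and a target component's position.
; Tick measures travel and moves the mesh at Speed, swapping endpoints on arrival and pausing for three seconds.
; During each pause it disables the Box collision, never re-enabled here, and assigns Floor_Mesh to the mesh.
; DontStopMove is never called here, and the hide-mesh node is unconnected.
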(event EventBeginPlay
  (Variables|Default|SetStartLoaction (Variables|/Script/Engine.SceneComponent|GetRelativeLocation (Variables|Default|GetStaticMesh)))
  (Variables|Default|SetTargetLocation (Variables|/Script/Engine.SceneComponent|GetRelativeLocation (Variables|Default|GetTargetCompoent))))

(event Collision|EventActorBeginOverlap
  (params (OtherActor :type Actor%20Object%20Reference)))

(event EventTick
  (params (DeltaSeconds :type Float%20%28single-precision%29))
  (if (Variables|Default|GetIsWait)
    (CallFunction|WaitTimeCheck DeltaSeconds)
    (Collision|SetCollisionEnabled (Variables|Default|GetBox) "NoCollision")
    (Components|StaticMesh|SetStaticMesh (Variables|Default|GetStaticMesh) "/Engine/EditorMeshes/AssetViewer/Floor_Mesh.Floor_Mesh")
    (else
      (CallFunction|LenthCheck)
      (bind _ischange (CallFunction|Shulfe))
      (Variables|Default|SetIsWait _ischange)
      (CallFunction|MoveUpdate DeltaSeconds))))

(fn ConstructionScript)

(fn MoveUpdate
  (params (DaltaTime :type Float%20%28double-precision%29))
  (Transformation|SetRelativeLocation (Variables|Default|GetStaticMesh) (+ (Variables|/Script/Engine.SceneComponent|GetRelativeLocation (Variables|Default|GetStaticMesh)) (* (Math|Vector|Normalize (- (Variables|Default|GetTargetLocation) (Variables|Default|GetStartLoaction))) (* (Variables|Default|GetSpeed) DaltaTime))) false false))

(fn Shulfe
  (bind _travlled (Variables|Default|GetTravlled))
  (bind _length (Variables|Default|GetLength))
  (bind _returnvalue (>= _travlled _length))
  (if _returnvalue
    (Variables|Default|SetTempLoaction (Variables|Default|GetStartLoaction))
    (Variables|Default|SetStartLoaction (Variables|Default|GetTargetLocation))
    (Variables|Default|SetTargetLocation (Variables|Default|GetTempLoaction))
    (return _returnvalue)
    (else
      (return false))))

(fn LenthCheck
  (Variables|Default|SetLength (Math|Vector|VectorLength (- (Variables|Default|GetTargetLocation) (Variables|Default|GetStartLoaction))))
  (Variables|Default|SetTravlled (Math|Vector|VectorLength (- (Variables|/Script/Engine.SceneComponent|GetRelativeLocation (Variables|Default|GetStaticMesh)) (Variables|Default|GetStartLoaction)))))

(fn WaitTimeCheck
  (params (DeltaTime :type Float%20%28double-precision%29))
  (bind _output_get (Variables|Default|SetAccTime (+ (Variables|Default|GetAccTime) DeltaTime)))
  (if (>= _output_get 3.0)
    (Variables|Default|SetIsWait false)
    (Variables|Default|SetAccTime 0.0)))

(fn DontStopMove
  (params (DeltaTime :type Float%20%28double-precision%29))
  (CallFunction|WaitTimeCheck DeltaTime)
  (CallFunction|LenthCheck)
  (bind _ischange (CallFunction|Shulfe))
  (Variables|Default|SetIsWait _ischange)
  (CallFunction|MoveUpdate 0.0))