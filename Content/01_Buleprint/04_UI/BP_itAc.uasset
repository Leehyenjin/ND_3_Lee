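; BP_itAc is an interaction actor that destroys an assigned monster actor and itself once an interaction is held long enough.
; While OnInterection is set, Tick accumulates time toward MaxTime and resets it otherwise, feeding the remaining fraction to its InterctionUI widget.
; SetMon supplies the monster reference, and debug prints report whether that reference is valid when assigned and upon completion.
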(event Custom|SetMon
  (params (MonsterActor :type Actor%20Object%20Reference))
  (bind _output_get (Variables|Default|SetMonsterActor MonsterActor))
  (Utilities|IsValid _output_get
    (:Is%20Valid
      (Development|PrintString "SettingComplite"))
    (:Is%20Not%20Valid
      (Development|PrintString "SettingFail"))))

(event EventBeginPlay)

(event Collision|EventActorBeginOverlap
  (params (OtherActor :type Actor%20Object%20Reference)))

(event EventTick
  (params (DeltaSeconds :type Float%20%28single-precision%29))
  (bind _monsteractor (Variables|Default|GetMonsterActor))
  (if (Variables|Default|GetOnInterection)
    (Variables|Default|SetAccTime (+ (Variables|Default|GetAccTime) DeltaSeconds))
    (else
      (Variables|Default|SetAccTime 0.0)))
  (bind _asinterction_ui (Utilities|Casting|CastToInterctionUI (UserInterface|GetWidget (Variables|Default|GetWidget))))
  (Default|SetPer _asinterction_ui (- 1.0 (/ (Variables|Default|GetAccTime) (Variables|Default|GetMaxTime))))
  (if (>= (Variables|Default|GetAccTime) (Variables|Default|GetMaxTime))
    (Utilities|IsValid _monsteractor
      (:Is%20Valid
        (Development|PrintString "Mon")
        (Actor|DestroyActor _monsteractor)
        (Actor|DestroyActor))
      (:Is%20Not%20Valid
        (Development|PrintString "NO")))))

(fn ConstructionScript)