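; Moving cube actor that shuttles between its mesh's start and a target component's location while periodically firing a spawned actor.
; Tick moves the mesh in relative space, swapping endpoints once travelled distance reaches path length.
; IsWaitCube selects non-stop or waiting movement, but Shulfe always returns false, so the endpoint pause never triggers.
; A separate cooldown timer spawns the configured Class ahead of the mesh.
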(event EventBeginPlay
  (Variables|Default|SetStartLocation (Variables|/Script/Engine.SceneComponent|GetRelativeLocation (Variables|Default|GetStaticMesh)))
  (Variables|Default|SetTargetLocation (Variables|/Script/Engine.SceneComponent|GetRelativeLocation (Variables|Default|GetTargetComponent))))

(event Collision|EventActorBeginOverlap
  (params (OtherActor :type Actor%20Object%20Reference)))

(event EventTick
  (params (DeltaSeconds :type Float%20%28single-precision%29))
  (Utilities|FlowControl|Sequence
    (:then_0
      (if (Variables|Default|GetIsWaitCube)
        (CallFunction|DontStopMove DeltaSeconds)
        (else
          (CallFunction|WaitMove DeltaSeconds))))
    (:then_1
      (CallFunction|ComputeShootingTime DeltaSeconds))))

(fn ConstructionScript)

(fn MoveUpdate
  (params (DeltaTime :type Float%20%28double-precision%29))
  ;[1 1 1] 이동
  (Transformation|SetRelativeLocation (Variables|Default|GetStaticMesh) (+ (Variables|/Script/Engine.SceneComponent|GetRelativeLocation (Variables|Default|GetStaticMesh)) (* (Math|Vector|Normalize (- (Variables|Default|GetTargetLocation) (Variables|Default|GetStartLocation))) (* (Variables|Default|GetSpeed) DeltaTime))) false false))

(fn LenthCheck
  ;[1 1 1] 가야할 거리
  (Variables|Default|SetLength (Math|Vector|VectorLength (- (Variables|Default|GetTargetLocation) (Variables|Default|GetStartLocation))))
  ;[1 1 1] 가고있는 거리
  (Variables|Default|SetTravelled (Math|Vector|VectorLength (- (Variables|/Script/Engine.SceneComponent|GetRelativeLocation (Variables|Default|GetStaticMesh)) (Variables|Default|GetStartLocation)))))

(fn Shulfe
  ;[1 1 1] 위치 셔플 바꾸기
  (if (>= (Variables|Default|GetTravelled) (Variables|Default|GetLength))
    (Variables|Default|SetTempLocation (Variables|Default|GetStartLocation))
    (Variables|Default|SetStartLocation (Variables|Default|GetTargetLocation))
    (Variables|Default|SetTargetLocation (Variables|Default|GetTempLocation))
    (return false)
    (else
      (return false))))

(fn WaitTimeCheck
  (params (DaltaTime :type Float%20%28double-precision%29))
  (bind _output_get (Variables|Default|SetAccTime (+ (Variables|Default|GetAccTime) DaltaTime)))
  (if (>= _output_get 3.0)
    (Variables|Default|SetIsWait false)
    (Variables|Default|SetAccTime 0.0)))

(fn WaitMove
  (params (DaltaTime :type Float%20%28double-precision%29))
  (if (Variables|Default|GetIsWait)
    (CallFunction|WaitTimeCheck 0.0)
    (else
      (CallFunction|LenthCheck)
      (bind _ischange (CallFunction|Shulfe))
      (Variables|Default|SetIsWait _ischange)
      (CallFunction|MoveUpdate DaltaTime))))

(fn DontStopMove
  (params (DaltaTime :type Float%20%28double-precision%29))
  (CallFunction|LenthCheck)
  (CallFunction|Shulfe)
  (CallFunction|MoveUpdate DaltaTime))

(fn Shooting
  (bind _staticmesh (Variables|Default|GetStaticMesh))
  (bind _returnvalue (Transformation|GetWorldTransform _staticmesh))
  (Game|SpawnActorfromClass (Variables|Default|Getclass) (Math|Transform|MakeTransform (+ (.location _returnvalue) (* (Math|Vector|GetForwardVector _staticmesh) 8e+01)) (.rotation _returnvalue) (.scale _returnvalue)) "Undefined" "MultiplyWithRoot" 0 0))

(fn ComputeShootingTime
  (params (DaltaTime :type Float%20%28double-precision%29))
  (bind _output_get (Variables|Default|SetProjectileAccTime (+ (Variables|Default|GetProjectileAccTime) DaltaTime)))
  (if (>= _output_get (Variables|Default|GetProjectileShootingCoolTime))
    (CallFunction|Shooting)
    (Variables|Default|SetProjectileAccTime 0.0)))