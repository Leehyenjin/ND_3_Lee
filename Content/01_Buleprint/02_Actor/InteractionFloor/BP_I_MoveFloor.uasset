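; Interaction floor whose static mesh shuttles between its starting position and a target component's position, gated on a BP_Base_character overlapping its box.
; Tick and both overlap events share the cast checks feeding GoMove and DontStopMove.
; These step the mesh at constant speed, swapping endpoints once traveled distance reaches the path length.
; A three-second wait timer exists but is effectively bypassed, since GoMove routes waiting into DontStopMove.
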(event OnComponentBeginOverlap(Box)
  (params (OverlappedComponent :type Primitive%20Component%20Object%20Reference) (OtherActor :type Actor%20Object%20Reference) (OtherComp :type Primitive%20Component%20Object%20Reference) (OtherBodyIndex :type Integer) (bFromSweep :type Boolean) (SweepResult :type Hit%20Result%20Structure%20%28by%20ref%29))
  (bind _asbp_base_character (Utilities|Casting|CastToBP_Base_character OtherActor))
  (Utilities|IsValid _asbp_base_character
    (:Is%20Valid
      (CallFunction|GoMove (stale EventTick DeltaSeconds)))))

(event OnComponentEndOverlap(Box)
  (params (OverlappedComponent :type Primitive%20Component%20Object%20Reference) (OtherActor :type Actor%20Object%20Reference) (OtherComp :type Primitive%20Component%20Object%20Reference) (OtherBodyIndex :type Integer))
  (bind _asbp_base_character (Utilities|Casting|CastToBP_Base_character OtherActor))
  (Utilities|IsValid _asbp_base_character
    (:Is%20Valid
      (CallFunction|DontStopMove (stale EventTick DeltaSeconds)))))

(event EventBeginPlay
  (Variables|Default|SetStartLoaction (Variables|/Script/Engine.SceneComponent|GetRelativeLocation (Variables|Default|GetStaticMesh)))
  (Variables|Default|SetTargetLocation (Variables|/Script/Engine.SceneComponent|GetRelativeLocation (Variables|Default|GetTargetCompoent))))

(event Collision|EventActorBeginOverlap
  (params (OtherActor :type Actor%20Object%20Reference)))

(event EventTick
  (params (DeltaSeconds :type Float%20%28single-precision%29))
  (Utilities|FlowControl|Sequence
    (:then_0
      (bind _asbp_base_character (Utilities|Casting|CastToBP_Base_character (stale OnComponentBeginOverlap(Box) OtherActor)))
      (Utilities|IsValid _asbp_base_character
        (:Is%20Valid
          (CallFunction|GoMove DeltaSeconds))))
    (:then_1
      (bind _asbp_base_character_2 (Utilities|Casting|CastToBP_Base_character (stale OnComponentEndOverlap(Box) OtherActor)))
      (Utilities|IsValid _asbp_base_character_2
        (:Is%20Valid
          (CallFunction|DontStopMove DeltaSeconds))))))

(fn ConstructionScript)

(fn MoveUpdate
  (params (DaltaTime :type Float%20%28double-precision%29))
  (Transformation|SetRelativeLocation (Variables|Default|GetStaticMesh) (+ (Variables|/Script/Engine.SceneComponent|GetRelativeLocation (Variables|Default|GetStaticMesh)) (* (Math|Vector|Normalize (- (Variables|Default|GetTargetLocation) (Variables|Default|GetStartLoaction))) (* (Variables|Default|GetSpeed) DaltaTime))) false false))

(fn Shulfe
  (bind _travlled (Variables|Default|GetTravlled))
  (bind _length (Variables|Default|GetLength))
  (bind _returnvalue (>= _travlled _length))
  (if _returnvalue
    (Variables|Default|SetTempLoaction (Variables|Default|GetStartLoaction))
    (Variables|Default|SetStartLoaction (Variables|Default|GetTargetLocation))
    (Variables|Default|SetTargetLocation (Variables|Default|GetTempLoaction))
    (return _returnvalue)
    (else
      (return false))))

(fn LenthCheck
  (Variables|Default|SetLength (Math|Vector|VectorLength (- (Variables|Default|GetTargetLocation) (Variables|Default|GetStartLoaction))))
  (Variables|Default|SetTravlled (Math|Vector|VectorLength (- (Variables|/Script/Engine.SceneComponent|GetRelativeLocation (Variables|Default|GetStaticMesh)) (Variables|Default|GetStartLoaction)))))

(fn WaitTimeCheck
  (params (DeltaTime :type Float%20%28double-precision%29))
  (bind _output_get (Variables|Default|SetAccTime (+ (Variables|Default|GetAccTime) DeltaTime)))
  (if (>= _output_get 3.0)
    (Variables|Default|SetIsWait false)
    (Variables|Default|SetAccTime 0.0)))

(fn DontStopMove
  (params (DeltaTime :type Float%20%28double-precision%29))
  (CallFunction|LenthCheck)
  (CallFunction|Shulfe)
  (CallFunction|MoveUpdate DeltaTime))

(fn GoMove
  (params (DalteTime :type Float%20%28double-precision%29))
  (if (Variables|Default|GetIsWait)
    (CallFunction|DontStopMove DalteTime)
    (else
      (CallFunction|WaitMove DalteTime))))

(fn WaitMove
  (params (DeltaTime :type Float%20%28double-precision%29))
  (if (Variables|Default|GetIsWait)
    (CallFunction|WaitTimeCheck 0.0)
    (else
      (CallFunction|LenthCheck)
      (bind _ischange (CallFunction|Shulfe))
      (Variables|Default|SetIsWait _ischange)
      (CallFunction|MoveUpdate DeltaTime))))